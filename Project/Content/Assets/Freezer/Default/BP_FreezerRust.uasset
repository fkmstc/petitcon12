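; Freezer goal actor that stays hidden until the player's polar bear has collected every individual item.
; A custom event counts true flags in the character's FreezerIndividualStruct and, when all are set, reveals the mesh with custom depth.
; Entering the Box afterwards sets PolarBearCast, which the Level Blueprint reads to play a movie.
; A Sequencer-triggered event then shows the NextStage widget with mouse input for the title transition.
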(event OnComponentBeginOverlap(Box)
  (params (OverlappedComponent :type Primitive%20Component%20Object%20Reference) (OtherActor :type Actor%20Object%20Reference) (OtherComp :type Primitive%20Component%20Object%20Reference) (OtherBodyIndex :type Integer) (bFromSweep :type Boolean) (SweepResult :type Hit%20Result%20Structure%20%28by%20ref%29))
  ;[1 1 1] すべて集め終わってBox内に入ったとき、ムービー再生フラグ
  ; レベルブループリントにて判断
  (Utilities|Casting|CastToPolarBearCharacter OtherActor)
  (if (Variables|Default|GetbIndividualComplete)
    (Variables|Default|SetbPolarBearCast true)))

(event Custom|CustomEventMoveTitle
  (bind _returnvalue (Game|GetPlayerController 0))
  ;[1 1 1] シーケンサー内でのフラグ処理
  ; タイトル遷移
  (bind _returnvalue_2 (UserInterface|CreateWidget "/Game/Widget/UI_Item/nextstage.NextStage_C"))
  (UserInterface|Viewport|AddtoViewport _returnvalue_2 0)
  (Variables|/Script/Engine.PlayerController|SetbShowMouseCursor _returnvalue true)
  (Input|SetInputModeGameandUI _returnvalue 0 "DoNotLock" true))

(event Custom|CustomEventStructReference
  (bind _freezer_mesh (Variables|Default|GetFreezer_mesh))
  ;[1 1 1] Struct参照
  (Variables|Default|Setcount 0)
  (bind _aspolar_bear_character (Utilities|Casting|CastToPolarBearCharacter (Game|Player|GetPlayerPawn 0)))
  ;[1 1 1] Struct内がすべてTrueかどうかの判断
  (for _array_element (.individual_get_boolean (Variables|/Game/PolarBear/PolarBearCharacter.PolarBearCharacter_C|GetFreezerIndividualStruct _aspolar_bear_character))
    (if (Math|Boolean|Equal(Boolean) _array_element true)
      (bind _output_get (Variables|Default|Setcount (+ (Variables|Default|Getcount) 1)))
      ;[1 0.1863 0.1664] CountUp
      (Development|PrintString (Utilities|String|ToString(Integer) _output_get))))
  (if (== (Variables|Default|Getcount) (Utilities|Array|Length (.individual_get_boolean (Variables|/Game/PolarBear/PolarBearCharacter.PolarBearCharacter_C|GetFreezerIndividualStruct _aspolar_bear_character))))
    ;[1 1 1] メッシュの表示
    (Development|SetHiddeninGame _freezer_mesh false false)
    (Rendering|SetRenderCustomDepth _freezer_mesh true)
    (Variables|Default|SetbIndividualComplete true)))

(event EventBeginPlay
  ;[1 1 1] 始めは非表示
  (Development|SetHiddeninGame (Variables|Default|GetFreezer_mesh) true false))

(fn ConstructionScript)