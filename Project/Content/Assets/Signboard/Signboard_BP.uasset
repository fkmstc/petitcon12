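; Signboard actor that lets the player bring up an instruction widget, described in comments as the controls guide, when nearby.
; Tick shows its widget component, a "Y" prompt icon, only within range of the player.
; A box overlap with PolarBearCharacter sets Active, gating CustomEventQkey, which toggles the screen widget created on BeginPlay along with cursor and input mode.
; Closing reverses the widget's Start animation and delays before removing it.
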(event OnComponentBeginOverlap(Box)
  (params (OverlappedComponent :type Primitive%20Component%20Object%20Reference) (OtherActor :type Actor%20Object%20Reference) (OtherComp :type Primitive%20Component%20Object%20Reference) (OtherBodyIndex :type Integer) (bFromSweep :type Boolean) (SweepResult :type Hit%20Result%20Structure%20%28by%20ref%29))
  ;[1 1 1] Boxに入ったときActiveTrue
  ; 抜けたときFalse
  (Utilities|Casting|CastToPolarBearCharacter OtherActor)
  (Variables|Default|SetbActive true))

(event OnComponentEndOverlap(Box)
  (params (OverlappedComponent :type Primitive%20Component%20Object%20Reference) (OtherActor :type Actor%20Object%20Reference) (OtherComp :type Primitive%20Component%20Object%20Reference) (OtherBodyIndex :type Integer))
  ;[1 1 1] Boxに入ったときActiveTrue
  ; 抜けたときFalse
  (Utilities|Casting|CastToPolarBearCharacter OtherActor)
  (Variables|Default|SetbActive false))

(event Custom|CustomEventQkey
  (bind _returnvalue (Game|GetPlayerController 0))
  (bind _returnvalue_2 (Game|GetPlayerController 0))
  (bind _widgetykey (Variables|Default|GetWidgetYKey))
  ;[1 1 1] カスタムイベント：ActiveがTrueの時，Widget（操作方法）を表示
  (if (Variables|Default|GetbActive)
    (if (UserInterface|Viewport|IsinViewport (Variables|Default|GetWidgetYKey))
      (Variables|/Script/Engine.PlayerController|SetbShowMouseCursor _returnvalue_2 false)
      (Input|SetInputModeGameOnly _returnvalue_2)
      (Class|UserWidget|PlayAnimationReverse _widgetykey (Variables|/Game/Widget/Widget_Signboard.Widget_Signboard_C|GetStart _widgetykey) 1.0)
      (Utilities|FlowControl|Delay 1.0)
      (Widget|RemovefromParent (Variables|Default|GetWidgetYKey))
      (else
        (Variables|/Script/Engine.PlayerController|SetbShowMouseCursor _returnvalue true)
        (Input|SetInputModeGameandUI _returnvalue 0 "DoNotLock" true)
        (UserInterface|Viewport|AddtoViewport (Variables|Default|GetWidgetYKey) 0)))))

(event EventBeginPlay
  ;[1 1 1] Widgetをセット
  (bind _returnvalue (UserInterface|CreateWidget "/Game/Widget/Widget_Signboard.Widget_Signboard_C"))
  (Variables|Default|SetWidgetYKey _returnvalue))

(event EventTick
  (params (DeltaSeconds :type Float%20%28single-precision%29))
  (bind _widget (Variables|Default|GetWidget))
  ;[1 1 1] キャラクターとの距離が遠かった時(1000以下)，「Y」アイコン（Widget）を表示
  ; それより遠い場合非表示
  (if (<= (Transformation|GetDistanceTo (Game|Player|GetPlayerPawn 0)) 1e+03)
    (Development|SetHiddeninGame _widget false false)
    (else
      (Development|SetHiddeninGame _widget true false))))

(fn ConstructionScript)